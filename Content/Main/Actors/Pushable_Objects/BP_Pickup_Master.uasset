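; Master pickup Blueprint for items a character can carry, driven by interaction interface events.
; Sphere overlaps notify the other actor, while in-range events add or remove a Pickup button on the player's interaction widget.
; Starting interaction turns the mesh's collision responses to Ignore and snaps the item to the character's PickupSocket.
; Stopping clears the character and detaches in world space, without restoring collision.
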(event OnComponentBeginOverlap(Sphere)
  (params (OverlappedComponent :type Primitive%20Component%20Object%20Reference) (OtherActor :type Actor%20Object%20Reference) (OtherComp :type Primitive%20Component%20Object%20Reference) (OtherBodyIndex :type Integer) (bFromSweep :type Boolean) (SweepResult :type Hit%20Result%20Structure%20%28by%20ref%29))
  (Class|ALSCharacterBPI|BPIOverlappedInc(Message) OtherActor))

(event OnComponentEndOverlap(Sphere)
  (params (OverlappedComponent :type Primitive%20Component%20Object%20Reference) (OtherActor :type Actor%20Object%20Reference) (OtherComp :type Primitive%20Component%20Object%20Reference) (OtherBodyIndex :type Integer))
  (Class|ALSCharacterBPI|BPIOverlappedDec(Message) OtherActor))

(event EventBPIStartInteract
  (params (Character :type Character%20Object%20Reference))
  (Variables|Default|SetCharacter Character)
  (CallFunction|SnapItemtoActor))

(event EventBPIStopInteract
  (params (Character :type Character%20Object%20Reference))
  (Variables|Default|SetCharacter 0)
  (Transformation|DetachFromActor "KeepWorld" "KeepWorld" "KeepWorld"))

(event EventBPIInteractinRange
  (bind _can_interact (Class|BPIPlayerController|BPIGetInteractionWidget(Message) (Game|GetPlayerController 0)))
  (Class|BPIWidgetButtons|AddButton(Message) _can_interact (Utilities|Struct|MakeDataTableRowHandle "/Game/Resources/InputAction_Widget/UI/DT_UniversalActions.DT_UniversalActions" "Pickup") "Pickup"))

(event EventBPIInteractOutRange
  (bind _can_interact (Class|BPIPlayerController|BPIGetInteractionWidget(Message) (Game|GetPlayerController 0)))
  (Class|BPIWidgetButtons|DeleteButton(Message) _can_interact "Pickup"))

(fn ConstructionScript)

(fn SnapItemtoActor
  (Collision|SetCollisionResponsetoAllChannels (Variables|Default|GetStaticMesh) "ECR_Ignore")
  (Transformation|AttachComponentToComponent (Variables|/Script/Engine.Character|GetMesh (Variables|Default|GetCharacter)) (Variables|Default|GetPickup%20Socket) "SnapToTarget" "SnapToTarget" "KeepWorld" true))

(fn BPICanInteract
  (return true))