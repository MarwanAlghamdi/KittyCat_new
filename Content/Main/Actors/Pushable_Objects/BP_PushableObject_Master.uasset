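; Master pushable object that the player can push from predefined points, joined by AI helper characters.
; Construction builds arrows and overlap spheres from transform arrays; when in range, a widget marks the nearest point.
; Interaction checks room, floor and line of sight with traces, then a timeline slides the player into place before BPC_PushComponent begins pushing.
; NPCs spawn for other unblocked points and are told to stop when interaction ends.
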(event Custom|On%20Overlap%20Start
  (params (OverlappedComponent :type Primitive%20Component%20Object%20Reference) (OtherActor :type Actor%20Object%20Reference) (OtherComp :type Primitive%20Component%20Object%20Reference) (OtherBodyIndex :type Integer) (bFromSweep :type Boolean) (SweepResult :type Hit%20Result%20Structure%20%28by%20ref%29))
  ;[0.2464 0.3971 0.401] Switch hide and show the closest indicator
  ;;[0.2969 0.2969 0.2969] Overlapping Start and end
  (Class|ALSCharacterBPI|BPIOverlappedInc(Message) OtherActor))

(event Custom|On%20Overlap%20End
  (params (OverlappedComponent :type Primitive%20Component%20Object%20Reference) (OtherActor :type Actor%20Object%20Reference) (OtherComp :type Primitive%20Component%20Object%20Reference) (OtherBodyIndex :type Integer))
  ;[0.2464 0.3971 0.401] Switch hide and show the closest indicator
  ;;[0.2969 0.2969 0.2969] Overlapping Start and end
  (Class|ALSCharacterBPI|BPIOverlappedDec(Message) OtherActor))

(event Custom|Move%20Player%20to%20Point
  (params (Target%20Transform :type Transform))
  (bind (_location _rotation) (Math|Transform|BreakTransform Target%20Transform))
  (bind _returnvalue (Transformation|GetActorLocation))
  (bind _returnvalue_2 (Game|GetPlayerCharacter 0))
  (bind (_x _y) (Math|Vector|BreakVector _returnvalue))
  (bind (_x_2 _y_2) (Math|Vector|BreakVector _location))
  (bind _returnvalue_3 (Math|Vector|MakeVector _x_2 _y_2 0.0))
  (bind _returnvalue_4 (Math|Vector|MakeVector _x _y 0.0))
  (bind _returnvalue_5 (Math|Rotator|FindLookatRotation _returnvalue_4 _returnvalue_3))
  (bind _returnvalue_6 (Math|Vector|GetForwardVector _returnvalue_5))
  (bind _returnvalue_7 (* _returnvalue_6 36.0))
  (bind _returnvalue_8 (+ _returnvalue_7 _location))
  ;[0.225 0.2384 0.2812] Move Player to point
  ;;[0.225 0.2384 0.2812] Stop Movement
  (Components|Movement|StopMovementImmediately (Variables|/Script/Engine.Character|GetCharacterMovement (Game|GetPlayerCharacter 0)))
  ;;[0.225 0.2384 0.2812] Interp movement to
  (Animation|Montage|PlayMontage (Variables|/Script/Engine.Character|GetMesh (Game|GetPlayerCharacter 0)) "/Game/Resources/AnimX/_Common/CatMannequin/Anim/Move/A_Cat_Move_Run_F_Montage.A_Cat_Move_Run_F_Montage" 1.2
    (:then
      (Input|DisableInput (Game|GetPlayerCharacter 0) (Game|GetPlayerController 0))
      (bind _lerp (Timeline|Timeline_MoveCharacter PlayFromStart)
        (:Update
          (Transformation|SetActorLocationAndRotation _returnvalue_2 (Math|Vector|Lerp(Vector) (Transformation|GetActorLocation _returnvalue_2) (Math|Vector|MakeVector (.x _returnvalue_8) (.y _returnvalue_8) (.z (Transformation|GetActorLocation (Game|GetPlayerCharacter 0)))) _lerp) (Math|Rotator|Lerp(Rotator) (Transformation|GetActorRotation _returnvalue_2) _rotation _lerp)))
        (:Finished
          ;;[0.225 0.2384 0.2812] Start Pushing
          (Default|BeginPush (Variables|Default|GetPush%20Component) self))))))

(event EventBPIInteractinRange
  (bind _widget (Variables|Default|GetWidget))
  ;[0.2464 0.3971 0.401] Switch hide and show the closest indicator
  (bind _index (CallFunction|FindtheClosestPointIndex (Transformation|GetActorLocation (Game|GetPlayerCharacter 0)) 5e+02))
  (bind _output_get (Variables|Default|SetClose%20Indicator%20idx _index))
  ;;[0.225 0.2384 0.2812] set Widget transform to the pushing
  (Rendering|SetVisibility _widget true false)
  (Class|WidgetComponent|SetTickMode _widget "Enabled")
  (Transformation|SetRelativeLocation _widget (+ (.Location (Math|Transform|BreakTransform (Utilities|Array|Get(acopy) (Variables|Default|GetPushTransforms) _output_get))) "0.000000,0.000000,10.000000") false false)
  (Transformation|SetRelativeRotation _widget (Math|Rotator|Delta(Rotator) (.Rotation (Math|Transform|BreakTransform (Utilities|Array|Get(acopy) (Variables|Default|GetPushTransforms) _output_get))) "0.000000,180.000000,0.000000") false false)
  (bind _can_interact (Class|BPIPlayerController|BPIGetInteractionWidget(Message) (Game|GetPlayerController 0)))
  (bind _returnvalue (Utilities|GetDataTableRow "/Game/Resources/InputAction_Widget/UI/DT_UniversalActions.DT_UniversalActions" "Interact")
    (:then
      (Class|BPIWidgetButtons|AddButton(Message) _can_interact (Utilities|Struct|MakeDataTableRowHandle "/Game/Resources/InputAction_Widget/UI/DT_UniversalActions.DT_UniversalActions" (Utilities|String|StringToName (Utilities|String|ToString(Text) (.displayname _returnvalue)))) (.displayname _returnvalue)))))

(event EventBPIStartInteract
  (params (Character :type Character%20Object%20Reference))
  ;[0.225 0.2384 0.2812] Hold Begins
  (CallFunction|HandleInteraction Character))

(event EventBPIInteractOutRange
  ;[0.2464 0.3971 0.401] Switch hide and show the closest indicator
  (Utilities|HideIndicator))

(event EventBPIStopInteract
  (params (Character :type Character%20Object%20Reference))
  ;[0.225 0.2384 0.2812] Hold Begins
  (Default|EndPush (Variables|Default|GetPush%20Component))
  (Variables|Default|Setpushing%20idx -1)
  (Utilities|DespawnNPCs))

(event EventBeginPlay
  ;[0.2969 0.2969 0.2969] Whenever we collide with them will fire
  (Utilities|FlowControl|Sequence
    (:then_0
      (for _array_element (Variables|Default|GetSphere%20Collisions)
        (Collision|AssignOnComponentEndOverlap _array_element (EventDispatchers|CreateEvent :!event Custom|On%20Overlap%20End))
        (Collision|AssignOnComponentBeginOverlap _array_element (EventDispatchers|CreateEvent :!event Custom|On%20Overlap%20Start))))))

(fn ConstructionScript
  (Utilities|FlowControl|Sequence
    (:then_0
      (Utilities|Array|Clear (Variables|Default|GetDecals))
      (for _array_element (Variables|Default|GetPushTransforms)
        (AddComponent|AddArrowComponent false _array_element)))
    (:then_2
      (Utilities|Array|Clear (Variables|Default|GetSphere%20Collisions))
      (for _array_element_2 (Variables|Default|GetPush%20Indicator%20Collisions)
        (bind _returnvalue (AddComponent|AddSphereComponent false _array_element_2))
        (Utilities|Array|Add (Variables|Default|GetSphere%20Collisions) _returnvalue)))))

(fn HandleInteraction
  (params (Character :type Character%20Object%20Reference))
  (Utilities|HideIndicator)
  (CallFunction|SpawnNpcs)
  ;[0.2969 0.2969 0.2969] Start Pushing
  (CallFunction|MovePlayertoPoint (Variables|Default|GetTarget%20Transform)))

(fn UpdateInteractionMsg
  (params (Text :type Text)))

(fn FindtheClosestPointIndex
  (params (Character%20Location :type Vector) (Push%20Range :type Float%20%28double-precision%29))
  (for (_array_element _array_index) (Variables|Default|GetPushTransforms)
    (LocalVariables|SetCurrent%20Idx _array_index)
    (LocalVariables|SetCurrent%20Distance%20 (Class|KismetMathLibrary|VectorDistance2DSquared (Math|Transform|TransformLocation (Transformation|GetActorTransform) (.Location (Math|Transform|BreakTransform _array_element))) Character%20Location))
    (if (< (LocalVariables|GetCurrent%20Distance%20) (Math|Float|Square Push%20Range)) ; Whithing the range ?
      (if (or (< (LocalVariables|GetCurrent%20Distance%20) (LocalVariables|GetBetter%20Distance%20)) (< (LocalVariables|GetBetter%20Distance%20Idx) 0))
        (LocalVariables|SetBetter%20Distance%20Idx (LocalVariables|GetCurrent%20Idx))
        (LocalVariables|SetBetter%20Distance%20 (LocalVariables|GetCurrent%20Distance%20)))))
  (return (LocalVariables|GetBetter%20Distance%20Idx)))

(fn GetCharacterNewTransform
  (params (Index :type Integer) (Character :type Character%20Object%20Reference))
  (bind _returnvalue (Transformation|GetActorTransform))
  (bind _pushtransforms (Variables|Default|GetPushTransforms))
  (bind _output (Utilities|Array|Get(acopy) _pushtransforms Index))
  (bind _returnvalue_2 (Math|Transform|ComposeTransforms _output _returnvalue))
  (bind (_location _rotation) (Math|Transform|BreakTransform _returnvalue_2))
  (return (Math|Transform|MakeTransform _location _rotation)))

(fn UpdateCharacterRotation
  (params (InTransform :type Transform%20%28by%20ref%29))
  (bind (_location _rotation) (Math|Transform|BreakTransform InTransform))
  (bind _returnvalue (Game|GetPlayerCharacter 0))
  (bind _returnvalue_2 (Transformation|GetActorRotation _returnvalue))
  (bind (_roll _pitch) (Math|Rotator|BreakRotator _returnvalue_2))
  (Transformation|SetActorRotation _returnvalue (Math|Interpolation|RInterpTo _returnvalue_2 (Math|Rotator|MakeRotator _roll _pitch (.Yaw (Math|Rotator|BreakRotator _rotation))) (Utilities|Time|GetWorldDeltaSeconds) (Math|Float|Lerp 4.0 1e+01 (Math|Float|MapRangeClamped (Math|Float|Max(Float) (- (Class|KismetMathLibrary|VectorDistance2DSquared (Transformation|GetActorLocation _returnvalue) _location) 1.6e+03) 0.0) 3040.3 1e+02 0.0 1.0))))
  (return 0.0 (Math|Rotator|Delta(Rotator) _returnvalue_2 _rotation)))

(fn CanInteract?
  (params (Character :type Character%20Object%20Reference))
  (bind _returnvalue (Transformation|GetActorLocation Character))
  (bind _capsulecomponent (Variables|/Script/Engine.Character|GetCapsuleComponent Character))
  (Utilities|IsValid Character
    (:Is%20Valid
      (bind _output_get (Variables|Default|SetPush%20Component (Actor|GetComponentbyClass Character "/Game/Main/Components/BPC_PushComponent.BPC_PushComponent_C")))
      (Utilities|IsValid _output_get
        (:Is%20Valid
          (bind _index (CallFunction|FindtheClosestPointIndex (Transformation|GetActorLocation Character) (Variables|Default|GetPush%20Range)))
          (bind _output_get_2 (LocalVariables|Setclose%20idx _index))
          (if (>= _output_get_2 0)
            (bind _output_get_3 (LocalVariables|SetNew%20Character%20Transform (CallFunction|GetCharacterNewTransform (LocalVariables|Getclose%20idx) Character)))
            (Variables|Default|SetTarget%20Transform _output_get_3)
            ;[0.1779 0.2188 0.15] Check for obstacles
            (bind _outhit (Collision|CapsuleTraceByChannel (+ (.location (LocalVariables|GetNew%20Character%20Transform)) "0.000000,0.000000,50.000000") (- (.location (LocalVariables|GetNew%20Character%20Transform)) "0.000000,0.000000,500.000000") (Components|Capsule|GetScaledCapsuleRadius _capsulecomponent) (Components|Capsule|GetScaledCapsuleHalfHeight _capsulecomponent) "TraceTypeQuery1" false (Utilities|Array|MakeArray Character) "ForDuration" true "(R=0.154099,G=0.177083,B=0.138171,A=1.000000)" "(R=0.000000,G=1.000000,B=0.000000,A=1.000000)" 1.0))
            (if (.bInitialOverlap (Collision|BreakHitResult _outhit))
              (|SiriusPrintStringFormatted "No Room To Push this object" true true "(R=1.000000,G=0.000000,B=0.082829,A=1.000000)")
              (return false)
              (elif (< (Class|CharacterMovementComponent|GetWalkableFloorZ (Variables|/Script/Engine.Character|GetCharacterMovement Character)) (.Z (Math|Vector|BreakVector (.ImpactNormal (Collision|BreakHitResult _outhit)))))
                (bind (_outhit_2 _returnvalue_2) (Collision|LineTraceByChannel _returnvalue (Math|Vector|MakeVector (.X (Math|Vector|BreakVector (Math|Transform|TransformLocation (Transformation|GetActorTransform) (.Location (Math|Transform|BreakTransform (Utilities|Array|Get(acopy) (Variables|Default|GetPushTransforms) (LocalVariables|Getclose%20idx))))))) (.Y (Math|Vector|BreakVector (Math|Transform|TransformLocation (Transformation|GetActorTransform) (.Location (Math|Transform|BreakTransform (Utilities|Array|Get(acopy) (Variables|Default|GetPushTransforms) (LocalVariables|Getclose%20idx))))))) (.Z (Math|Vector|BreakVector _returnvalue))) "TraceTypeQuery1" false (Utilities|Array|MakeArray Character) "ForDuration" true "(R=0.664557,G=1.000000,B=0.855931,A=1.000000)" "(R=0.000000,G=1.000000,B=0.000000,A=1.000000)" 0.5))
                (if _returnvalue_2
                  (|SiriusPrintStringFormatted "Something hitting between character and the object Which is {a}" (.HitActor (Collision|BreakHitResult _outhit_2)) true true "(R=1.000000,G=0.000000,B=0.082829,A=1.000000)")
                  (return false)
                  (else
                    (Variables|Default|Setpushing%20idx (LocalVariables|Getclose%20idx))
                    (return true)))
                (else
                  (|SiriusPrintStringFormatted "Floor Is not walkable" true true "(R=1.000000,G=0.000000,B=0.082829,A=1.000000)")
                  (return false))))
            (else
              (|SiriusPrintStringFormatted "No Pushing Points whithin {r} radius" (Variables|/Game/Main/Components/BPC_PushComponent.BPC_PushComponent_C|GetPush%20Range (Variables|Default|GetPush%20Component)) true true "(R=1.000000,G=0.000000,B=0.082829,A=1.000000)")
              (return false))))
        (:Is%20Not%20Valid
          (|SiriusPrintStringFormatted "Push Component is invalid" true true "(R=1.000000,G=0.000000,B=0.082829,A=1.000000)")
          (return false))))
    (:Is%20Not%20Valid
      (|SiriusPrintStringFormatted "Character is invalid" true true "(R=1.000000,G=0.000000,B=0.082829,A=1.000000)")
      (return false))))

(fn SpawnNpcs
  (bind _returnvalue (Transformation|GetActorTransform))
  (bind _asbp_smokey (Utilities|Casting|CastToBP_Smokey (Game|Player|GetPlayerPawn 0)))
  (LocalVariables|Setcharacter_ _asbp_smokey)
  (for (_array_element _array_index) (Variables|Default|GetPushTransforms)
    (Utilities|FlowControl|Sequence
      (:then_0
        (if (!= _array_index (Variables|Default|Getpushing%20idx)) ; skip the pushing point
          (bind _returnvalue_2 (Collision|SphereTraceForObjects (Math|Transform|TransformLocation (Transformation|GetActorTransform) (+ (.location _array_element) (* (CallFunction|InvertVector (Math|Vector|GetForwardVector (.rotation _array_element))) 4e+01))) (Math|Transform|TransformLocation (Transformation|GetActorTransform) (+ (.location _array_element) (* (CallFunction|InvertVector (Math|Vector|GetForwardVector (.rotation _array_element))) 4e+01))) 35.0 (Utilities|Array|MakeArray "ObjectTypeQuery1") false (Utilities|Array|MakeArray self) "ForDuration"))
          (if _returnvalue_2
            (Utilities|Array|Add (LocalVariables|GetBlocked%20idx) _array_index)
            (else
              (bind (_outhit _returnvalue_3) (Collision|LineTraceByChannel (Math|Transform|TransformLocation _returnvalue (.location _array_element)) (Math|Transform|TransformLocation _returnvalue (+ (.location _array_element) (* (CallFunction|InvertVector (Math|Vector|GetForwardVector (.rotation _array_element))) (Variables|Default|GetSpawn%20Distance)))) "TraceTypeQuery1" false 0 "ForDuration"))
              (bind _returnvalue_4 (Game|SpawnActorfromClass "/Game/Resources/AdvancedLocomotionV4/Blueprints/CharacterLogic/ALS_AnimMan_CharacterBP.ALS_AnimMan_CharacterBP_C" (Math|Transform|MakeTransform (Math|Transform|TransformLocation (Transformation|GetActorTransform) (+ (.location _array_element) (* (CallFunction|InvertVector (Math|Vector|GetForwardVector (.rotation _array_element))) (Math|Float|SelectFloat (CallFunction|GetDistance(Hit) _outhit) (Variables|Default|GetSpawn%20Distance) _returnvalue_3)))) (.rotation _array_element) "0.400000,0.400000,0.400000") "Undefined" "OverrideRootScale" 0 0))
              (Utilities|Array|Add (Variables|Default|GetSpawned%20npcs) _returnvalue_4)
              (Default|AIStartPushing _returnvalue_4 (Math|Transform|TransformLocation (Transformation|GetActorTransform) (+ (.location _array_element) (* (CallFunction|InvertVector (Math|Vector|GetForwardVector (.rotation _array_element))) 4e+01))) self))))))))

(fn BPICanInteract
  (bind _asbp_smokey (Utilities|Casting|CastToBP_Smokey (Game|GetPlayerCharacter 0)))
  (switch Utilities|FlowControl|Switch|SwitchonE_MovementState (Variables|/Game/Main/Character/BP_Pawn_Master.BP_Pawn_Master_C|GetState%20-%20Movement%20State _asbp_smokey)
    (:NewEnumerator0
      _)
    (:NewEnumerator1
      _)
    (:NewEnumerator2
      (if (Default|IsHoldingObject (Variables|/Game/Main/Character/BP_Pawn_Master.BP_Pawn_Master_C|GetBPC_PushComponent _asbp_smokey))
        _
        (else
          (bind _return_value (CallFunction|CanInteract? (Game|GetPlayerCharacter 0)))
          (return _return_value))))
    (:NewEnumerator3
      _))
  (return false))