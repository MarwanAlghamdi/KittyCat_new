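; Actor component that lets a BP_Pawn_Master character push objects around.
; BeginPush attaches the character to the object's mesh, ignores its pawn collision, enables tick and updates the button prompt; EndPush reverses this.
; Tick interpolates character-relative input using the object's speed factor and offsets the object without sweep, carrying the attached character along.
; CanMove blocks movement using look-ahead sphere traces at each push transform and a box trace of the mesh bounds.
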(event EventBeginPlay
  (bind _asbp_pawn_master (Utilities|Casting|CastToBP_Pawn_Master (Components|GetOwner)))
  (Variables|Default|SetCharacter _asbp_pawn_master))

(event EventTick
  (params (DeltaSeconds :type Float%20%28single-precision%29))
  (bind _returnvalue (CallFunction|GetDeltaLocation true true true))
  (Variables|Default|SetCurrent%20Yaw%20Rotation (.yaw (Transformation|GetActorRotation (Variables|Default|GetCharacter))))
  (Variables|Default|GetCurrent%20Pushable%20Object
    (:then
      ;[0.225 0.2384 0.2812] Interp the input speed
      (bind _output_get (Variables|Default|SetInterp%20Input%20Direction (Math|Interpolation|VInterpTo (Variables|Default|GetInterp%20Input%20Direction) _returnvalue (Utilities|Time|GetWorldDeltaSeconds) (Math|Float|SelectFloat 0.0 (* (Variables|/Game/Main/Actors/Pushable_Objects/BP_PushableObject_Master.BP_PushableObject_Master_C|GetSpeed%20Factor (Variables|Default|GetCurrent%20Pushable%20Object)) (Variables|Default|GetPush%20Speed%20Interp)) false))))
      (Variables|Default|SetCurrent%20Pushing%20speed (Math|Vector|VectorLengthXY _output_get))
      (bind _returnvalue_2 (CallFunction|CanMove _returnvalue))
      (if _returnvalue_2
        _
        (else
          (Variables|Default|SetInterp%20Input%20Direction "0, 0, 0")))
      (Transformation|AddActorWorldOffset (Variables|Default|GetCurrent%20Pushable%20Object) (Variables|Default|GetInterp%20Input%20Direction)))
    (:else)))

(fn BeginPush
  (params (PushableObject :type BP%20Pushable%20Object%20Master%20Object%20Reference))
  (Default|BPISetOverlayState (Variables|Default|GetCharacter) "NewEnumerator3")
  (Components|Tick|SetComponentTickEnabled true)
  (bind _output_get (Variables|Default|SetCurrent%20Pushable%20Object PushableObject))
  (Collision|SetCollisionResponsetoChannel (Variables|/Game/Main/Actors/Pushable_Objects/BP_PushableObject_Master.BP_PushableObject_Master_C|GetMainMesh _output_get) "ECC_Pawn" "ECR_Ignore")
  (Transformation|AttachComponentToComponent (Variables|Default|GetCharacter) (Variables|/Game/Main/Actors/Pushable_Objects/BP_PushableObject_Master.BP_PushableObject_Master_C|GetMainMesh _output_get) "None" "KeepWorld" "KeepWorld" "KeepWorld" false)
  ;[0.225 0.2384 0.2812] - Change State
  ; - Display a button to indicate exiting
  (Input|EnableInput (Game|GetPlayerCharacter 0) (Game|GetPlayerController 0))
  (bind _can_interact (Class|BPIPlayerController|BPIGetInteractionWidget(Message) (Game|GetPlayerController 0)))
  (bind _returnvalue (Utilities|GetDataTableRow "/Game/Resources/InputAction_Widget/UI/DT_UniversalActions.DT_UniversalActions" "Interact")
    (:then
      (Class|BPIWidgetButtons|DeleteButton(Message) _can_interact (.holddisplayname _returnvalue))
      (Class|BPIWidgetButtons|AddButton(Message) _can_interact (Utilities|Struct|MakeDataTableRowHandle "/Game/Resources/InputAction_Widget/UI/DT_UniversalActions.DT_UniversalActions" (Utilities|String|StringToName (Utilities|String|ToString(Text) (.displayname _returnvalue)))) (Variables|Default|GetUI%20Button%20Text)))))

(fn IsHoldingObject
  (return (Utilities|IsValid (Variables|Default|GetCurrent%20Pushable%20Object))))

(fn EndPush
  (Default|BPISetOverlayState (Variables|Default|GetCharacter) "NewEnumerator0")
  (Variables|/Game/Main/Actors/Pushable_Objects/BP_PushableObject_Master.BP_PushableObject_Master_C|SetCan%20Check%20Collision (Variables|Default|GetCurrent%20Pushable%20Object) true)
  (Collision|SetCollisionResponsetoChannel (Variables|/Game/Main/Actors/Pushable_Objects/BP_PushableObject_Master.BP_PushableObject_Master_C|GetMainMesh (Variables|Default|GetCurrent%20Pushable%20Object)) "ECC_Pawn" "ECR_Block")
  (Variables|Default|SetCurrent%20Pushable%20Object 0)
  (Transformation|DetachFromActor (Variables|Default|GetCharacter) "KeepWorld" "KeepWorld" "KeepWorld")
  (Components|Tick|SetComponentTickEnabled false)
  (Input|SetIgnoreMoveInput (Pawn|GetController (Variables|Default|GetCharacter)) false)
  (bind _can_interact (Class|BPIPlayerController|BPIGetInteractionWidget(Message) (Game|GetPlayerController 0)))
  (Class|BPIWidgetButtons|DeleteButton(Message) _can_interact (Variables|Default|GetUI%20Button%20Text))
  (Variables|Default|SetInterp%20Input%20Direction "0, 0, 0")
  (Variables|Default|SetCurrent%20Pushing%20speed 0.0)
  (Input|EnableInput (Game|GetPlayerCharacter 0) (Game|GetPlayerController 0)))

(fn GetDeltaLocation
  (params (Invert%20X :type Boolean) (Invert%20Y :type Boolean) (Flip%20XY :type Boolean))
  (bind _character (Variables|Default|GetCharacter))
  (bind _move_fwd_bwd (Variables|/Game/Main/Character/BP_Pawn_Master.BP_Pawn_Master_C|GetMove%20FWD/BWD _character))
  (bind _move_r_l (Variables|/Game/Main/Character/BP_Pawn_Master.BP_Pawn_Master_C|GetMove%20R/L _character))
  (Variables|Default|SetIs%20Moving%20an%20object (or (!= _move_fwd_bwd 0.0) (!= 0.0 _move_r_l)))
  (LocalVariables|SetX (Math|Float|SelectFloat _move_fwd_bwd (CallFunction|InvertFloat _move_fwd_bwd) Invert%20X))
  (LocalVariables|SetY (Math|Float|SelectFloat _move_r_l (CallFunction|InvertFloat _move_r_l) Invert%20Y))
  (if (and (== (Math|Float|Absolute(Float) (LocalVariables|GetX)) 1.0) (== (Math|Float|Absolute(Float) (LocalVariables|GetY)) 1.0))
    (LocalVariables|SetX (/ (LocalVariables|GetX) 2.0))
    (LocalVariables|SetY (/ (LocalVariables|GetY) 2.0)))
  (if Flip%20XY
    (bind _save_value (Utilities|TemporarilySaved (LocalVariables|GetY))
      (:%20
        (LocalVariables|SetY (LocalVariables|GetX))
        (LocalVariables|SetX _save_value))))
  (return (+ (* (* (Transformation|GetActorRightVector (Variables|Default|GetCharacter)) (LocalVariables|GetY)) (* (Utilities|Time|GetWorldDeltaSeconds) (Variables|Default|GetPush%20Speed))) (* (* (Transformation|GetActorForwardVector (Variables|Default|GetCharacter)) (LocalVariables|GetX)) (* (Utilities|Time|GetWorldDeltaSeconds) (Variables|Default|GetPush%20Speed))))))

(fn CalculateHeight
  (params (Push%20Location :type Vector))
  (bind _character (Variables|Default|GetCharacter))
  (bind _output_get (Variables|Default|SetPush%20Height (- (Components|Capsule|GetScaledCapsuleHalfHeight (Variables|/Script/Engine.Character|GetCapsuleComponent _character)) (.Z (Math|Vector|BreakVector (- Push%20Location (Transformation|GetActorLocation _character)))))))
  (Variables|Default|SetPush%20Height%20type (select (> (Math|Float|Absolute(Float) _output_get) 4e+01) 0 0))
  (|SiriusPrintStringFormatted (Utilities|String|ToString(Float) _output_get)))

(fn CanMove
  (params (Movement%20Direction :type Vector))
  (bind _returnvalue (* Movement%20Direction 2e+01))
  (bind _current_pushable_object (Variables|Default|GetCurrent%20Pushable%20Object))
  (bind _current_pushable_object_2 (Variables|Default|GetCurrent%20Pushable%20Object))
  (bind _returnvalue_2 (Transformation|GetActorTransform _current_pushable_object))
  (bind _mainmesh (Variables|/Game/Main/Actors/Pushable_Objects/BP_PushableObject_Master.BP_PushableObject_Master_C|GetMainMesh _current_pushable_object_2))
  (bind (_origin _boxextent) (Collision|GetComponentBounds _mainmesh))
  (bind (_x _y _z) (Math|Vector|BreakVector _origin))
  (bind _returnvalue_3 (+ _z 3.0))
  (bind _returnvalue_4 (Math|Vector|MakeVector _x _y _returnvalue_3))
  (bind _returnvalue_5 (+ _returnvalue _returnvalue_4))
  (for _array_element (Variables|/Game/Main/Actors/Pushable_Objects/BP_PushableObject_Master.BP_PushableObject_Master_C|GetPushTransforms _current_pushable_object)
    (bind _returnvalue_6 (Collision|SphereTraceForObjects (+ (* Movement%20Direction 2e+01) (+ (Math|Transform|TransformLocation _returnvalue_2 (.location _array_element)) (* 35.0 (Math|Transform|TransformDirection _returnvalue_2 (CallFunction|InvertVector (Math|Vector|GetForwardVector (.rotation _array_element))))))) (+ (* Movement%20Direction 2e+01) (+ (Math|Transform|TransformLocation _returnvalue_2 (.location _array_element)) (* 35.0 (Math|Transform|TransformDirection _returnvalue_2 (CallFunction|InvertVector (Math|Vector|GetForwardVector (.rotation _array_element))))))) 3e+01 (Utilities|Array|MakeArray "ObjectTypeQuery1" "ObjectTypeQuery7") false (Utilities|Array|MakeArray (Variables|Default|GetCurrent%20Pushable%20Object) (Variables|Default|GetCharacter)) "ForOneFrame"))
    (if _returnvalue_6
      (return false)))
  ;[0.225 0.2384 0.2812] Box to check overlaps
  (bind _returnvalue_7 (Class|KismetSystemLibrary|BoxTraceSingleforObjects _returnvalue_5 _returnvalue_5 _boxextent "0, 0, 0" (Utilities|Array|MakeArray "ObjectTypeQuery1") false (Utilities|Array|MakeArray (Variables|Default|GetCurrent%20Pushable%20Object) 0) "ForOneFrame" true))
  (if _returnvalue_7
    (return false)
    (else
      (return true))))