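; BP_Smokey is a character Blueprint that handles interacting with objects, commented as pushing them.
; The Interact input toggles interaction with InteractableObject through Blueprint Interface messages, checking whether it can interact before starting.
; Debug keys add, clear or force-add button prompts on the player controller's interaction widget, using rows from DT_UniversalActions.
; Punch input only prints a placeholder string.
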(event Input|EnhancedActionEvents|EnhancedInputActionIA_Punch
  (params (ActionValue :type Boolean) (ElapsedSeconds :type Float%20%28double-precision%29) (TriggeredSeconds :type Float%20%28double-precision%29) (InputAction :type Input%20Action%20Object%20Reference :default "/Game/Main/InputActions/inputs/IA_Punch.IA_Punch"))
  (:Started
    (Development|PrintString "Hello")))

(event Input|EnhancedActionEvents|EnhancedInputActionIA_Interact
  (params (ActionValue :type Boolean) (ElapsedSeconds :type Float%20%28double-precision%29) (TriggeredSeconds :type Float%20%28double-precision%29) (InputAction :type Input%20Action%20Object%20Reference :default "/Game/Main/InputActions/inputs/IA_Interact.IA_Interact"))
  (bind _interactable_object (Variables|Default|GetInteractable%20Object))
  ;[0.225 0.2384 0.2812] Interact - Push objects
  (:Started
    (if (Variables|Default|GetInteracting)
      (Class|BPIInteract|BPIStopInteract(Message) (Variables|Default|GetInteractable%20Object) self)
      (Variables|Default|SetInteracting false)
      (else
        (bind _can_interact (Class|BPIInteract|BPICanInteract(Message) _interactable_object))
        (if _can_interact
          (Class|BPIInteract|BPIStartInteract(Message) _interactable_object self)
          (Variables|Default|SetInteracting true)
          (else
            (Development|PrintString "Interaction Could not be happend." true true "(R=1.000000,G=0.000000,B=0.065548,A=1.000000)")))))))

(event EventBeginPlay
  (|CallParentFunction))

(event Input|KeyboardEvents|X
  (params (Key :type Key%20Structure :default "None"))
  ;[0.225 0.2384 0.2812] Widget debugging
  (:Pressed
    (Utilities|FlowControl|FlipFlop
      (:A
        (bind _returnvalue (Utilities|GetDataTableRow "/Game/Resources/InputAction_Widget/UI/DT_UniversalActions.DT_UniversalActions" "Interact")
          (:then
            (bind _can_interact (Class|BPIPlayerController|BPIGetInteractionWidget(Message) (Game|GetPlayerController 0)))
            (Class|BPIWidgetButtons|ForceAddButton(Message) _can_interact (Utilities|Struct|MakeDataTableRowHandle "/Game/Resources/InputAction_Widget/UI/DT_UniversalActions.DT_UniversalActions" (Utilities|TexttoString (.DisplayName (Utilities|Struct|BreakCommonInputActionDataBase _returnvalue)))) "Interact"))))
      (:B
        (bind _returnvalue_2 (Utilities|GetDataTableRow "/Game/Resources/InputAction_Widget/UI/DT_UniversalActions.DT_UniversalActions" "Forward")
          (:then
            (bind _can_interact_2 (Class|BPIPlayerController|BPIGetInteractionWidget(Message) (Game|GetPlayerController 0)))
            (Class|BPIWidgetButtons|ForceAddButton(Message) _can_interact_2 (Utilities|Struct|MakeDataTableRowHandle "/Game/Resources/InputAction_Widget/UI/DT_UniversalActions.DT_UniversalActions" (Utilities|TexttoString (.DisplayName (Utilities|Struct|BreakCommonInputActionDataBase _returnvalue_2)))) "Forward")))))))

(event Input|KeyboardEvents|Z
  (params (Key :type Key%20Structure :default "None"))
  ;[0.225 0.2384 0.2812] Widget debugging
  (:Pressed
    (bind _can_interact (Class|BPIPlayerController|BPIGetInteractionWidget(Message) (Game|GetPlayerController 0)))
    (Class|BPIWidgetButtons|ClearButtons(Message) _can_interact)))

(event Input|KeyboardEvents|C
  (params (Key :type Key%20Structure :default "None"))
  ;[0.225 0.2384 0.2812] Widget debugging
  (:Pressed
    (bind _returnvalue (Utilities|GetDataTableRow "/Game/Resources/InputAction_Widget/UI/DT_UniversalActions.DT_UniversalActions" "Interact")
      (:then
        (bind _can_interact (Class|BPIPlayerController|BPIGetInteractionWidget(Message) (Game|GetPlayerController 0)))
        (Class|BPIWidgetButtons|AddButton(Message) _can_interact (Utilities|Struct|MakeDataTableRowHandle "/Game/Resources/InputAction_Widget/UI/DT_UniversalActions.DT_UniversalActions" (Utilities|TexttoString (.DisplayName (Utilities|Struct|BreakCommonInputActionDataBase _returnvalue)))) (Utilities|Text|ToText(String) (|SiriusFormatString "{random} = Interact" (Math|Random|RandomInteger 50))))))))

(fn ConstructionScript
  (|CallParentFunction))