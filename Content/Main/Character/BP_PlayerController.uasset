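; Player controller that sets game-only input, creates the debug overlay and interaction widgets, and initializes the custom camera manager.
; On possess, it passes the pawn to BP_CamManager.
; Number keys and Tab toggle debug flags such as HUD, traces, shapes and slomo, and one key also adds or removes the overlay.
; Interface functions expose these flags and the interaction widget, reporting character info only while the overlay menu is closed.
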(event EventBeginPlay
  (Input|SetInputModeGameOnly self false)
  ;[0.225 0.2384 0.2812] Debug Widget
  (bind _returnvalue (UserInterface|CreateWidget "/Game/Main/UI/Debug/W_Debug.W_Debug_C" self))
  (bind _output_get (Variables|Default|SetOverlay%20Widget _returnvalue))
  (UserInterface|Viewport|AddtoViewport _output_get 0)
  (bind _returnvalue_2 (UserInterface|CreateWidget "/Game/Main/UI/Button/W_UI_Interactions.W_UI_Interactions_C" self))
  (bind _output_get_2 (Variables|Default|SetInteraction%20widget _returnvalue_2))
  (UserInterface|Viewport|AddtoViewport _output_get_2 0))

(event EventPossess
  (params (PossessedPawn :type Pawn%20Object%20Reference))
  ;[1 1 1] Setup Camera
  (bind _asbp_cam_manager (Utilities|Casting|CastToBP_CamManager (Variables|Default|GetPlayerCameraManager)))
  (Default|OnPossess _asbp_cam_manager PossessedPawn))

(event Input|KeyboardEvents|1
  (params (Key :type Key%20Structure :default "None"))
  ;[0.2961 0 0] Debug Keys
  (:Pressed
    (Variables|Default|SetDebug%20View (not (Variables|Default|GetDebug%20View)))))

(event Input|KeyboardEvents|Tab
  (params (Key :type Key%20Structure :default "None"))
  ;[0.2961 0 0] Debug Keys
  (:Pressed
    (Variables|Default|SetShow%20HUD (not (Variables|Default|GetShow%20HUD)))))

(event Input|KeyboardEvents|2
  (params (Key :type Key%20Structure :default "None"))
  ;[0.2961 0 0] Debug Keys
  (:Pressed
    (Variables|Default|SetShow%20Traces (not (Variables|Default|GetShow%20Traces)))))

(event Input|KeyboardEvents|4
  (params (Key :type Key%20Structure :default "None"))
  ;[0.2961 0 0] Debug Keys
  (:Pressed
    (Variables|Default|SetShow%20Layer%20Colors (not (Variables|Default|GetShow%20Layer%20Colors)))))

(event Input|KeyboardEvents|3
  (params (Key :type Key%20Structure :default "None"))
  ;[0.2961 0 0] Debug Keys
  (:Pressed
    (Variables|Default|SetShow%20Debug%20Shapes (not (Variables|Default|GetShow%20Debug%20Shapes)))))

(event Input|KeyboardEvents|5
  (params (Key :type Key%20Structure :default "None"))
  ;[0.2961 0 0] Debug Keys
  (:Pressed
    (Variables|Default|SetSlomo (not (Variables|Default|GetSlomo)))))

(event Input|KeyboardEvents|6
  (params (Key :type Key%20Structure :default "None"))
  ;[0.2961 0 0] Debug Keys
  (:Pressed
    (Variables|Default|SetShow%20Character%20Info (not (Variables|Default|GetShow%20Character%20Info)))))

(event Input|KeyboardEvents|7
  (params (Key :type Key%20Structure :default "None"))
  ;[0.2961 0 0] Debug Keys
  (:Pressed
    (Variables|Default|SetOverlay%20Menu%20Open (not (Variables|Default|GetOverlay%20Menu%20Open)))))

(event Input|KeyboardEvents|0
  (params (Key :type Key%20Structure :default "None"))
  (bind _overlay_widget (Variables|Default|GetOverlay%20Widget))
  ;[0.2961 0 0] Debug Keys
  (:Pressed
    (bind _isa (Utilities|FlowControl|FlipFlop)
      (:A
        (Variables|Default|SetOverlay%20Menu%20Open _isa)
        (UserInterface|Viewport|AddtoViewport _overlay_widget 0))
      (:B
        (Variables|Default|SetOverlay%20Menu%20Open _isa)
        (Widget|RemovefromParent _overlay_widget)))))

(fn ConstructionScript)

(fn BPIGetDebugInfo
  (return 0 (Variables|Default|GetDebug%20View) (Variables|Default|GetShow%20HUD) (Variables|Default|GetShow%20Traces) (Variables|Default|GetShow%20Debug%20Shapes) (Variables|Default|GetShow%20Layer%20Colors) (Variables|Default|GetSlomo) (and (Variables|Default|GetShow%20Character%20Info) (not (Variables|Default|GetOverlay%20Menu%20Open)))))

(fn BPIGetInteractionWidget
  (return (Variables|Default|GetInteraction%20widget)))